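; BP_MotionController is a VR actor that carries a pistol and moves at a constant speed along a fixed forward axis.
; BeginPlay sets floor tracking origin, and Tick offsets the actor's location without sweep.
; The right trigger draws a debug line trace from FirePos, whose result is unused, then plays the fire animation and spawns a BP_Bullet there.
; The head collision overlap event is an empty stub.
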(event OnComponentBeginOverlap(headCol)
  (params (OverlappedComponent :type Primitive%20Component%20Object%20Reference) (OtherActor :type Actor%20Object%20Reference) (OtherComp :type Primitive%20Component%20Object%20Reference) (OtherBodyIndex :type Integer) (bFromSweep :type Boolean) (SweepResult :type Hit%20Result%20Structure%20%28by%20ref%29)))

(event EventBeginPlay
  (Class|HeadMountedDisplayFunctionLibrary|SetTrackingOrigin "Floor"))

(event Collision|EventActorBeginOverlap
  (params (OtherActor :type Actor%20Object%20Reference)))

(event EventTick
  (params (DeltaSeconds :type Float%20%28single-precision%29))
  (Transformation|SetActorLocation (+ (* (* (Class|KismetMathLibrary|VectorForward) (Variables|Default|GetSpeed)) DeltaSeconds) (Transformation|GetActorLocation)) false false))

(event Input|ActionEvents|InputActionTriggerRight
  (params (Key :type Key%20Structure :default "None"))
  (bind _firepos (Variables|Default|GetFirePos))
  (bind _returnvalue (Transformation|GetWorldLocation _firepos))
  (:Pressed
    (Utilities|FlowControl|Sequence
      (:then_0
        (Collision|LineTraceByChannel _returnvalue (+ _returnvalue (* (Math|Vector|GetForwardVector (Transformation|GetWorldRotation _firepos)) (Variables|Default|GetBulletRange))) "TraceTypeQuery1" false 0 "ForDuration" true "(R=1.000000,G=0.880592,B=0.000000,A=1.000000)" "(R=1.000000,G=1.000000,B=1.000000,A=0.000000)"))
      (:then_1
        (Components|Animation|PlayAnimation (Variables|Default|GetPistol) "/Game/Assets/MilitaryWeapDark/Weapons/Anims/Fire_Pistol_S1.Fire_Pistol_S1" false)
        (Game|SpawnActorfromClass "/Game/BP_VR/BP_Bullet.BP_Bullet_C" (Transformation|GetWorldTransform _firepos) "AlwaysSpawn" 0 0)))))

(fn ConstructionScript)