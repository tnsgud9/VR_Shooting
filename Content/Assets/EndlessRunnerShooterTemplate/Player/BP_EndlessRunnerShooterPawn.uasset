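; Player pawn for an endless runner shooter template, layering weapon effects and a death reaction onto its parent class.
; Fire spawns a muzzle flash emitter and plays a gunshot sound, then calls the parent's Fire.
; GetProjectileSpawnLocation returns the Gun's Muzzle socket location, which also positions the flash.
; On player death, the Mesh switches to physics simulation.
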(event Custom|PlayMuzzleFlashAndSound
  (bind _projectilespawnlocation (CallFunction|GetProjectileSpawnLocation))
  (Effects|SpawnEmitteratLocation "/Game/Assets/EndlessRunnerShooterTemplate/ParticleEffects/P_MuzzleFlash.P_MuzzleFlash" _projectilespawnlocation)
  (Audio|PlaySoundatLocation "/Game/Assets/EndlessRunnerShooterTemplate/Sounds/CUE_Gunshot.CUE_Gunshot" (Transformation|GetWorldLocation (Variables|Character|GetMesh)) "0, 0, 0" 1.0 1.0 0.0 0 0 0))

(event EventFire
  (CallFunction|PlayMuzzleFlashandSound)
  (|CallParentFunction))

(event EventOnPlayerDied
  (Physics|SetSimulatePhysics (Variables|Character|GetMesh) true))

(fn ConstructionScript
  (|CallParentFunction))

(fn GetProjectileSpawnLocation
  (return (Transformation|GetSocketLocation (Variables|Default|GetGun) "Muzzle")))