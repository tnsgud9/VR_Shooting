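; BP_Corner is a SuperGrid tutorial level element that builds an adjustable inner or outer corner piece.
; Its construction script uses the Switch flag to choose corner meshes, rotation and scale axes.
; The HeightAndRotation transform is clamped, then its Z drives mesh scale and top-mesh offset while its rotation turns the Center component.
; All logic runs at construction, with no active gameplay events.
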(event EventBeginPlay)

(event Collision|EventActorBeginOverlap
  (params (OtherActor :type Actor%20Object%20Reference)))

(event EventTick
  (params (DeltaSeconds :type Float%20%28single-precision%29)))

(fn ConstructionScript
  (if (Variables|Settings|GetSwitch) ; Swap Inner and Outer corner
    _
    (else
      (Components|StaticMesh|SetStaticMesh "/Game/Assets/SuperGrid/StarterPack/Source/Meshes/SuperGrid_CylinderQuarter.SuperGrid_CylinderQuarter")
      (Components|StaticMesh|SetStaticMesh "/Game/Assets/SuperGrid/StarterPack/Source/Meshes/SuperGrid_CornerOuter.SuperGrid_CornerOuter")
      (Transformation|AddRelativeRotation "90.000000,0.000000,0.000000" false false)))
  (Utilities|FlowControl|Sequence
    (:then_0
      (Variables|Settings|SetHeightAndRotation (Math|Transform|MakeTransform (Math|Vector|MakeVector (Math|Float|Clamp(Float) (.X (Math|Vector|BreakVector (.location (Variables|Settings|GetHeightAndRotation)))) -1e+02 2e+02) (Math|Float|Clamp(Float) (.Y (Math|Vector|BreakVector (.location (Variables|Settings|GetHeightAndRotation)))) -1e+02 2e+02) (Math|Float|Clamp(Float) (.Z (Math|Vector|BreakVector (.location (Variables|Settings|GetHeightAndRotation)))) 1e+02 1e+05)) (.rotation (Variables|Settings|GetHeightAndRotation)) (.scale (Variables|Settings|GetHeightAndRotation)))) ; Calculate location and set rotation& scale
    )
    (:then_1
      (Transformation|SetRelativeScale3D (Math|Vector|SelectVector (Math|Vector|MakeVector (- (/ (.z (.location (Variables|Settings|GetHeightAndRotation))) 1e+02) 1.0) 1.0 1.0) (Math|Vector|MakeVector 2.0 2.0 (- (/ (.z (.location (Variables|Settings|GetHeightAndRotation))) 1e+02) 1.0)) (Variables|Settings|GetSwitch))) ; Update Scale
    )
    (:then_2
      (Transformation|AddLocalOffset (Math|Vector|MakeVector 0.0 0.0 (- (.z (.location (Variables|Settings|GetHeightAndRotation))) 1e+02)) false false) ; Update position of the top mesh
    )
    (:then_3
      (Transformation|SetRelativeRotation (Variables|Default|GetCenter) (.rotation (Variables|Settings|GetHeightAndRotation)) false false) ; Rotate meshes according to "HeightAndRotation" variable
    )))