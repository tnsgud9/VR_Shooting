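; Shooting enemy that yaws its skeletal mesh toward the player every tick while alive.
; Warning-area overlap plays a crouch-to-idle animation unless IsFired is set, which this graph never does.
; Fire-area overlap by BP_MotionController spawns one BP_Bullet aimed at its head collider, without checking IsAlive.
; Die clears IsAlive and turns the mesh into a physics body, launched by an amplified impulse at the hit location.
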(event OnComponentBeginOverlap(WarningArea)
  (params (OverlappedComponent :type Primitive%20Component%20Object%20Reference) (OtherActor :type Actor%20Object%20Reference) (OtherComp :type Primitive%20Component%20Object%20Reference) (OtherBodyIndex :type Integer) (bFromSweep :type Boolean) (SweepResult :type Hit%20Result%20Structure%20%28by%20ref%29))
  (if (not (Variables|Default|GetisFired))
    (Components|Animation|PlayAnimation (Variables|Default|GetSkeletalMesh) "/Game/Assets/EndlessRunnerShooterTemplate/StarterContent/Mannequin/Animations/ThirdPerson_CrouchToIdle.ThirdPerson_CrouchToIdle" false)))

(event OnComponentBeginOverlap(FireArea)
  (params (OverlappedComponent :type Primitive%20Component%20Object%20Reference) (OtherActor :type Actor%20Object%20Reference) (OtherComp :type Primitive%20Component%20Object%20Reference) (OtherBodyIndex :type Integer) (bFromSweep :type Boolean) (SweepResult :type Hit%20Result%20Structure%20%28by%20ref%29))
  (bind _firepos (Variables|Default|GetFirePos))
  (bind _asbp_motion_controller (Utilities|Casting|CastToBP_MotionController OtherActor))
  (Game|SpawnActorfromClass "/Game/BP_VR/BP_Bullet.BP_Bullet_C" (Math|Transform|MakeTransform (Transformation|GetWorldLocation _firepos) (Math|Rotator|FindLookatRotation (Transformation|GetWorldLocation _firepos) (Transformation|GetWorldLocation (Variables|/Game/Blueprints/Virtual_Reality/BP_MotionController.BP_MotionController_C|GetheadCol _asbp_motion_controller))) "1.000000,1,1") "Undefined" 0 0))

(event Custom|Die
  (params (hitImpulse :type Vector) (hitLocation :type Vector))
  (Variables|Default|SetisAlive false)
  (Physics|SetSimulatePhysics (Variables|Default|GetSkeletalMesh) true)
  (Physics|AddImpulseatLocation (Variables|Default|GetSkeletalMesh) (* hitImpulse 1e+04) hitLocation "None"))

(event EventTick
  (params (DeltaSeconds :type Float%20%28single-precision%29))
  (bind _skeletalmesh (Variables|Default|GetSkeletalMesh))
  (bind _returnvalue (Transformation|GetWorldRotation _skeletalmesh))
  (bind (_roll _pitch) (Math|Rotator|BreakRotator _returnvalue))
  ;[1 1 1] Always look at player
  (if (Variables|Default|GetisAlive)
    (Transformation|SetWorldRotation (Variables|Default|GetSkeletalMesh) (Math|Rotator|MakeRotator _roll _pitch (+ (.Yaw (Math|Rotator|BreakRotator (Math|Rotator|FindLookatRotation (Transformation|GetWorldLocation (Variables|Default|GetSkeletalMesh)) (Transformation|GetActorLocation (Game|Player|GetPlayerPawn 0))))) -9e+01)) false false)))

(event Collision|EventActorBeginOverlap
  (params (OtherActor :type Actor%20Object%20Reference)))

(event EventBeginPlay
  (Variables|Default|SetisAlive true))

(fn ConstructionScript)