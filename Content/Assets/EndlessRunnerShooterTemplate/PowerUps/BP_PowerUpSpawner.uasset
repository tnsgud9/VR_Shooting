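; BP_PowerUpSpawner spawns a random power-up on its parent endless runner tile at BeginPlay, continuing only when its parent actor is a BP_TileBase.
; GetPowerUp makes a weighted random pick from the PowerUps map of classes to weights.
; A valid pick spawns at a random point inside the SpawnArea box, sized by the construction script, and receives the parent tile reference.
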(event EventBeginPlay
  (bind _spawnarea (Variables|Default|GetSpawnArea))
  ;[1 1 1] Spawn PowerUp
  (bind _asbp_tile_base (Utilities|Casting|CastToBP_TileBase (Actor|GetParentActor)))
  (Variables|Default|SetparentTile _asbp_tile_base)
  (bind _powerup (CallFunction|GetPowerUp))
  (if (Utilities|IsValidClass _powerup)
    (Game|SpawnActorfromClass _powerup (Math|Conversions|ToTransform(Vector) (Math|Random|RandomPointinBoundingBox (Transformation|GetWorldLocation _spawnarea) (Variables|/Script/Engine.BoxComponent|GetBoxExtent _spawnarea))) "Undefined" 0 (Variables|Default|GetparentTile) 0)))

(fn ConstructionScript
  (Components|Box|SetBoxExtent (Variables|Default|GetSpawnArea) (Variables|Default|GetspawnBoxExtend) true))

(fn GetPowerUp
  (bind _powerups (Variables|Default|GetpowerUps))
  ;[1 1 1] Get a random PowerUp using weighted random selection
  (bind _values (Utilities|Map|Values (Variables|Default|GetpowerUps)))
  (for _array_element _values
    (LocalVariables|SettotalWeight (+ _array_element (LocalVariables|GettotalWeight))))
  (LocalVariables|SetrandomWeight (Math|Random|RandomFloatinRange 0.0 (LocalVariables|GettotalWeight)))
  (bind _keys (Utilities|Map|Keys _powerups))
  (bind _array_element_2 (Utilities|Array|ForEachLoopwithBreak _keys :!label _label)
    (:LoopBody
      (LocalVariables|SetcurrentWeight (+ (.Value (Utilities|Map|Find _powerups _array_element_2)) (LocalVariables|GetcurrentWeight)))
      (if (<= (LocalVariables|GetrandomWeight) (LocalVariables|GetcurrentWeight))
        (LocalVariables|SetcurrentPowerUp _array_element_2)
        (goto _label Break)))
    (:Completed
      (return (LocalVariables|GetcurrentPowerUp)))))