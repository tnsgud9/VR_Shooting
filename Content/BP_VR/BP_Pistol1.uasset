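; BP_Pistol1 is a VR pistol that plays fire and reload animations and spawns bullets.
; On BeginPlay it enables player 0 input on its parent actor.
; The Fire event or right trigger spawns BP_Bullet at FirePos.
; Right thumbstick down reloads only when IsReload is already true, while a right-mouse test input reloads when it is false; both set it true and nothing here resets it.
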(event Custom|Fire
  (Components|Animation|PlayAnimation (Variables|Default|GetPistol) "/Game/Assets/MilitaryWeapDark/Weapons/Anims/Fire_Pistol_S1.Fire_Pistol_S1" false)
  (Game|SpawnActorfromClass "/Game/BP_VR/BP_Bullet.BP_Bullet_C" (Transformation|GetWorldTransform (Variables|Default|GetFirePos)) "AlwaysSpawn" 0 0))

(event EventBeginPlay
  (Input|EnableInput (Actor|GetParentActor) (Game|GetPlayerController 0)))

(event Collision|EventActorBeginOverlap
  (params (OtherActor :type Actor%20Object%20Reference)))

(event EventTick
  (params (DeltaSeconds :type Float%20%28single-precision%29)))

(event Input|ActionEvents|InputActionTriggerRight
  (params (Key :type Key%20Structure))
  (:Pressed
    (Components|Animation|PlayAnimation (Variables|Default|GetPistol) "/Game/Assets/MilitaryWeapDark/Weapons/Anims/Fire_Pistol_S1.Fire_Pistol_S1" false)
    (Game|SpawnActorfromClass "/Game/BP_VR/BP_Bullet.BP_Bullet_C" (Transformation|GetWorldTransform (Variables|Default|GetFirePos)) "AlwaysSpawn" 0 0)))

(event Input|ActionEvents|InputActionMouseRight
  (params (Key :type Key%20Structure))
  ;[1 1 1] Testing Field
  (:Pressed
    (if (Math|Boolean|Equal(Boolean) (Variables|Default|GetisReload) false)
      (Development|PrintString "Hello")
      (Variables|Default|SetisReload true)
      (Components|Animation|PlayAnimation (Variables|Default|GetPistol) "/Game/Assets/MilitaryWeapDark/Weapons/Anims/Reload_Pistol_W.Reload_Pistol_W" false))))

(event Input|AxisEvents|InputAxisThumbstickRightDown
  (params (AxisValue :type Float%20%28single-precision%29))
  (if (and (>= AxisValue 0.7) (Variables|Default|GetisReload))
    (Variables|Default|SetisReload true)
    (Components|Animation|PlayAnimation (Variables|Default|GetPistol) "/Game/Assets/MilitaryWeapDark/Weapons/Anims/Reload_Pistol_W.Reload_Pistol_W" false)))

(fn ConstructionScript)