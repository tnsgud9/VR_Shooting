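; Red enemy Blueprint, apparently for an endless runner shooter, that stands up and fires when its trigger areas are overlapped.
; Overlapping WarningArea plays a crouch-to-idle animation; overlapping FireArea spawns a bullet at FirePos aimed at the overlapping actor, with neither checking what overlapped.
; On death, the skeletal mesh turns ragdoll and takes a scaled-up impulse at the hit location.
; The player-area events are empty, and a player Die call is left unconnected.
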(event OnComponentBeginOverlap(WarningArea)
  (params (OverlappedComponent :type Primitive%20Component%20Object%20Reference) (OtherActor :type Actor%20Object%20Reference) (OtherComp :type Primitive%20Component%20Object%20Reference) (OtherBodyIndex :type Integer) (bFromSweep :type Boolean) (SweepResult :type Hit%20Result%20Structure%20%28by%20ref%29))
  ;[1 1 1] When stand up animation when player enters warning area
  (Components|Animation|PlayAnimation (Variables|Default|GetSkeletalMesh) "/Game/Assets/EndlessRunnerShooterTemplate/StarterContent/Mannequin/Animations/ThirdPerson_CrouchToIdle.ThirdPerson_CrouchToIdle" false))

(event OnComponentBeginOverlap(FireArea)
  (params (OverlappedComponent :type Primitive%20Component%20Object%20Reference) (OtherActor :type Actor%20Object%20Reference) (OtherComp :type Primitive%20Component%20Object%20Reference) (OtherBodyIndex :type Integer) (bFromSweep :type Boolean) (SweepResult :type Hit%20Result%20Structure%20%28by%20ref%29))
  (bind _firepos (Variables|Default|GetFirePos))
  (bind _returnvalue (Transformation|GetWorldLocation _firepos))
  (Game|SpawnActorfromClass "/Game/BP_VR/BP_Bullet.BP_Bullet_C" (Math|Transform|MakeTransform _returnvalue (Math|Rotator|FindLookatRotation _returnvalue (Transformation|GetActorLocation OtherActor))) "Undefined" 0 0))

(event EventPlayeronFireArea
  (params (endlessRunnerShooterBase :type BP%20Endless%20Runner%20Shooter%20Pawn%20Base%20Object%20Reference))
  ;[1 1 1] Shoot when player is in fire area
)

(event EventPlayeronWarningArea
  (params (EndlessRunnerShooterBase :type BP%20Endless%20Runner%20Shooter%20Pawn%20Base%20Object%20Reference))
  ;[1 1 1] When stand up animation when player enters warning area
)

(event EventOnDied
  (params (hitImpulse :type Vector :default "0, 0, 0") (hitLocation :type Vector :default "0, 0, 0"))
  ;[1 1 1] Activate ragdoll on dead
  (Physics|SetSimulatePhysics (Variables|Default|GetSkeletalMesh) true)
  (Physics|AddImpulseatLocation (Variables|Default|GetSkeletalMesh) (* hitImpulse 1e+04) hitLocation "None"))

(event EventBeginPlay)

(fn ConstructionScript
  (|CallParentFunction))